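; Secondary camera rig for the Gunslinger that follows a Father actor and mirrors its camera orientation.
; Each Tick, while Father is valid, the Scene component copies Father's root world transform without sweeping.
; SpringArm2 then takes its relative rotation from Father's CameraPitch and CameraYaw with zero roll, keeping the aim separate from the copied transform.
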(event EventTick
  (params (DeltaSeconds :type Float%20%28single-precision%29))
  (bind _father (Variables|Default|GetFather))
  (bind _father_2 (Variables|Default|GetFather))
  (if (Utilities|IsValid _father)
    (Transformation|SetWorldTransform (Variables|Default|GetScene) (Transformation|GetWorldTransform (Variables|/Script/Engine.Actor|GetRootComponent _father)) false false)
    (Transformation|SetRelativeRotation (Variables|Default|GetSpringArm2) (Math|Rotator|MakeRotator 0.0 (Variables|/Game/Gunslinger/Gunslinger_BP.Gunslinger_BP_C|GetCameraPitch _father_2) (Variables|/Game/Gunslinger/Gunslinger_BP.Gunslinger_BP_C|GetCameraYaw _father_2)) false false)))

(fn ConstructionScript)