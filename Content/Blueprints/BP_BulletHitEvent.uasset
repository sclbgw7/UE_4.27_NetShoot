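; Short-lived actor that resolves a bullet hit, fed the hit target, component, direction, location, normal and damage through Initialize.
; On its first Tick it plays an impact sound, then branches on the target.
; Hat-tagged components on Characters or HitableObjects get launched spinning with physics; other hits on those targets apply damage on the authority.
; All non-hat hits spawn particles and a randomly rolled decal, and the actor destroys itself after a brief delay.
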(event Custom|Initialize
  (params (Other :type Actor%20Object%20Reference) (Other%20Comp :type Primitive%20Component%20Object%20Reference) (BulletDir :type Vector) (HitLocation :type Vector) (Hit%20Normal :type Vector) (Damage :type Float%20%28single-precision%29) (Causer :type Actor%20Object%20Reference))
  (Variables|Default|SetOther Other)
  (Variables|Default|SetOtherComp Other%20Comp)
  (Variables|Default|SetBulletDir BulletDir)
  (Variables|Default|SetHitLocation HitLocation)
  (Variables|Default|SetHitNormal Hit%20Normal)
  (Variables|Default|SetDamage Damage)
  (Variables|Default|SetCauser Causer)
  (Variables|Default|SetInitialized true))

(event Custom|DelayedDestroy
  (Utilities|FlowControl|Delay 0.2)
  (Actor|DestroyActor))

(event EventTick
  (params (DeltaSeconds :type Float%20%28single-precision%29))
  (bind _other (Variables|Default|GetOther))
  (bind _hitnormal (Variables|Default|GetHitNormal))
  (bind _hitlocation (Variables|Default|GetHitLocation))
  (bind _othercomp (Variables|Default|GetOtherComp))
  (bind _returnvalue (* _hitnormal -1.0))
  (bind _returnvalue_2 (Math|Conversions|RotationFromXVector _returnvalue))
  (Utilities|FlowControl|DoOnce false
    (:Completed
      ;[0 1 0] Sound
      (Audio|PlaySoundatLocation "/Game/Sounds/SoundCue_Attentuated.SoundCue_Attentuated" (Variables|Default|GetHitLocation) "0, 0,0.000000" (Variables|Default|GetVolumeMultiplier) (Math|Random|RandomFloatinRange 0.8 1.2) 0.0 0 0 0)
      (Utilities|Casting|CastToCharacter _other
        (:then
          (if (Components|ComponentHasTag (Variables|Default|GetOtherComp) "Hat") :!label _label
            ;[1 1 1] Hit Hat
            (CallFunction|DelayedDestroy)
            (Physics|SetSimulatePhysics _othercomp true)
            (Physics|SetPhysicsLinearVelocity _othercomp (* (Variables|Default|GetBulletDir) 0.33) false "None")
            (Class|PrimitiveComponent|SetPhysicsAngularVelocityinDegrees _othercomp (Math|Vector|MakeVector (Math|Random|RandomFloatinRange -7.2e+02 7.2e+02) (Math|Random|RandomFloatinRange -7.2e+02 7.2e+02) (Math|Random|RandomFloatinRange -7.2e+02 7.2e+02)) false "None")
            ;[0 1 0] Sound
            (Audio|PlaySoundatLocation "/Game/Sounds/Randomize_01.Randomize_01" (Variables|Default|GetHitLocation) "0, 0, 0" (* (Variables|Default|GetVolumeMultiplier) 0.25) 1.0 0.0 0 0 0)
            (else
              ;[1 1 1] Hit Character or HitableObjects
              (Networking|SwitchHasAuthority
                (:Authority
                  (Game|Damage|ApplyDamage (Variables|Default|GetOther) (Variables|Default|GetDamage) (Game|GetInstigatorController) (Variables|Default|GetCauser)))
                (:Remote
                  _))
              (CallFunction|DelayedDestroy :!label _label_2)
              (Effects|SpawnEmitteratLocation "/Game/Effects/P_Hit.P_Hit" _hitlocation)
              (Rendering|Decal|SpawnDecalatLocation "/Game/Materials/M_BulletDecal.M_BulletDecal" "30.000000,5.000000,5.000000" _hitlocation (Math|Rotator|MakeRotator (Math|Random|RandomFloatinRange -1.8e+02 1.8e+02) (.pitch _returnvalue_2) (.yaw _returnvalue_2)) 9.0))))
        (:CastFailed
          (Utilities|Casting|CastToHitableObject _other
            (:then
              (goto _label))
            (:CastFailed
              (goto _label_2))))))))

(fn ConstructionScript)