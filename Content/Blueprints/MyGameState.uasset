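; Game state that decides the match outcome from player scores when the match ends.
; EndMatch scans PlayerArray for the top score and tie count, then sets each MyPlayerState's Winning to mark sole winner, tie or loss.
; It then calls QuitMatch on the player state of player controller 0.
; The OnRep handlers for GameStartTimer and RandomTimerValue1 are empty.
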(fn ConstructionScript)

(fn OnRepGameStartTimer)

(fn OnRepRandomTimerValue1)

(fn EndMatch
  ;[1 1 1] Get the winner
  (for _array_element (Variables|Default|GetPlayerArray)
    (bind _asmy_player_state (Utilities|Casting|CastToMyPlayerState _array_element))
    (if (> (Variables|/Game/Blueprints/MyPlayerState.MyPlayerState_C|GetPlayerScore _asmy_player_state) (LocalVariables|GetMaxScore))
      (LocalVariables|SetMaxNum 1)
      (LocalVariables|SetMaxScore (Variables|/Game/Blueprints/MyPlayerState.MyPlayerState_C|GetPlayerScore _asmy_player_state))
      (elif (== (Variables|/Game/Blueprints/MyPlayerState.MyPlayerState_C|GetPlayerScore _asmy_player_state) (LocalVariables|GetMaxScore))
        (Math|Integer|IncrementInt (LocalVariables|GetMaxNum)))))
  (for _array_element_2 (Variables|Default|GetPlayerArray)
    (bind _asmy_player_state_2 (Utilities|Casting|CastToMyPlayerState _array_element_2))
    (if (== (Variables|/Game/Blueprints/MyPlayerState.MyPlayerState_C|GetPlayerScore _asmy_player_state_2) (LocalVariables|GetMaxScore))
      (if (== (LocalVariables|GetMaxNum) 1)
        (Variables|/Game/Blueprints/MyPlayerState.MyPlayerState_C|SetWinning _asmy_player_state_2 2)
        (else
          (Variables|/Game/Blueprints/MyPlayerState.MyPlayerState_C|SetWinning _asmy_player_state_2 1)))
      (else
        (Variables|/Game/Blueprints/MyPlayerState.MyPlayerState_C|SetWinning _asmy_player_state_2 0))))
  (bind _asmy_player_state_3 (Utilities|Casting|CastToMyPlayerState (Variables|/Script/Engine.Controller|GetPlayerState (Game|GetPlayerController 0))))
  (Default|QuitMatch _asmy_player_state_3))