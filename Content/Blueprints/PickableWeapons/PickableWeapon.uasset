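; Pickable weapon actor that notifies nearby Gunslinger_BP pawns that it is available to pick up.
; Tick accumulates time and, each time it exceeds CheckInterval, runs a small sphere overlap at the weapon's location, filtered to Gunslinger_BP pawns.
; Each pawn found receives NewWeaponCanPick with this weapon as the argument, so detection uses throttled polling in place of overlap events.
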(event EventTick
  (params (DeltaSeconds :type Float%20%28single-precision%29))
  (bind _checkinterval (Variables|Default|GetCheckInterval))
  (bind _output_get (Variables|Default|SetTimer (+ DeltaSeconds (Variables|Default|GetTimer))))
  (if (> _output_get _checkinterval)
    (Variables|Default|SetTimer (- _output_get _checkinterval))
    (bind (_outactors _returnvalue) (Collision|SphereOverlapActors (Transformation|GetActorLocation) 1e+02 (Utilities|Array|MakeArray "ObjectTypeQuery3") "/Game/Gunslinger/Gunslinger_BP.Gunslinger_BP_C"))
    (if _returnvalue
      (for _array_element _outactors
        (bind _asgunslinger_bp (Utilities|Casting|CastToGunslinger_BP _array_element))
        (Default|NewWeaponCanPick _asgunslinger_bp self)))))

(fn ConstructionScript)