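; FlyingCube is an Actor Blueprint in the HitableObjects folder that moves a cube continuously along a circular path.
; Each Tick accumulates elapsed time and sets the Cube component's relative X and Y from sine and cosine of that time.
; MoveSpeed controls how fast it circles and MoveRange sets the radius.
; The file shows no hit handling, and the construction script is empty.
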(event EventTick
  (params (DeltaSeconds :type Float%20%28single-precision%29))
  (bind _moverange (Variables|Default|GetMoveRange))
  (bind _output_get (Variables|Default|SetTime (+ (Variables|Default|GetTime) DeltaSeconds)))
  (Transformation|SetRelativeLocation (Variables|Default|GetCube) (Math|Vector|MakeVector (* (Math|Trig|Sin(Radians) (* _output_get (Variables|Default|GetMoveSpeed))) _moverange) (* (Math|Trig|Cos(Radians) (* _output_get (Variables|Default|GetMoveSpeed))) _moverange) 0.0) false false))

(fn ConstructionScript)