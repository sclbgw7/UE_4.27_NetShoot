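; BP_Grenade is a physics-driven grenade actor that explodes on hitting a Character or when it nearly stops moving.
; Tick watches the Sphere's velocity after a short delay from BeginPlay, so a freshly spawned grenade does not detonate at once.
; Both triggers call Boom, which spawns a scaled-up P_Hit particle at the sphere, then destroy the actor; the explosion applies no damage.
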(event EventTick
  (params (DeltaSeconds :type Float%20%28single-precision%29))
  (if (> (- (Actor|GetGameTimeSinceCreation) (Variables|Default|GetStartTime)) 0.1)
    (bind _returnvalue (Physics|GetPhysicsLinearVelocity (Variables|Default|GetSphere) "None"))
    (if (< (Math|Vector|VectorLength _returnvalue) 2e+01)
      (CallFunction|Boom)
      (Actor|DestroyActor))))

(event EventBeginPlay
  (Variables|Default|SetStartTime (Actor|GetGameTimeSinceCreation)))

(event Collision|EventHit
  (params (MyComp :type Primitive%20Component%20Object%20Reference) (Other :type Actor%20Object%20Reference) (OtherComp :type Primitive%20Component%20Object%20Reference) (bSelfMoved :type Boolean) (HitLocation :type Vector :default "0, 0, 0") (HitNormal :type Vector :default "0, 0, 0") (NormalImpulse :type Vector :default "0, 0, 0") (Hit :type Hit%20Result%20Structure%20%28by%20ref%29))
  (Utilities|Casting|CastToCharacter Other)
  (CallFunction|Boom)
  (Actor|DestroyActor))

(fn ConstructionScript)

(fn Boom
  (Effects|SpawnEmitteratLocation "/Game/Effects/P_Hit.P_Hit" (Transformation|GetWorldLocation (Variables|Default|GetSphere)) "0, 0, 0" "10.000000,10.000000,10.000000"))